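; BP_Duck is the player-controlled 2D platformer duck, moving along X with Enhanced Input and facing its travel direction.
; Each tick it picks idle, run, jump or fall flipbooks from ground state and velocity.
; Landing on a BP_Trex destroys it and bounces the duck upward.
; It adds a Healthbar widget and tracks damage with debug prints, with F and R keys for testing health loss.
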(event `self.ReceiveTick`
  (params (DeltaSeconds :type "Float (single-precision)"))
  (`self.Update Animation`))

(event `self.ReceiveBeginPlay`
  (bind _asplayer_controller (cast `PlayerController` (`self.GetController`)))
  (`EnhancedInputSubsystemInterface.AddMappingContext` (pcsubsystem `EnhancedInputLocalPlayerSubsystem` _asplayer_controller) "/Game/blueprint/input/IMC_Platforming.IMC_Platforming" 0 (struct))
  (bind _returnvalue (`|CreateWidget` "/Game/UI/Healthbar.Healthbar_C"))
  (`UserWidget.AddToViewport` _returnvalue 0))

(event `EnhancedInput|/Game/blueprint/input/Actions/IA_Jump`
  (params (ActionValue :type Boolean) (ElapsedSeconds :type "Float (double-precision)") (TriggeredSeconds :type "Float (double-precision)") (InputAction :type "InputAction Object Reference" :default "/Game/blueprint/input/Actions/IA_Jump.IA_Jump"))
  (:`Started`
    (`self.Jump`))
  (:`Completed`
    (`self.StopJumping`)))

(event `Key|F`
  (params (Key :type "Key Structure"))
  (:`Pressed`
    (bind _output_get (set `self.Health` (`KismetMathLibrary.FClamp` (- (`self.Health`) 10.0) 0.0 100.0)))
    (`KismetSystemLibrary.PrintString` (`KismetStringLibrary.Conv_DoubleToString` _output_get))))

(event `EnhancedInput|/Game/blueprint/input/Actions/IA_Move`
  (params (ActionValue :type "Float (double-precision)") (ElapsedSeconds :type "Float (double-precision)") (TriggeredSeconds :type "Float (double-precision)") (InputAction :type "InputAction Object Reference" :default "/Game/blueprint/input/Actions/IA_Move.IA_Move"))
  (:`Triggered`
    (`self.AddMovementInput` (1.0 0.0 0.0) ActionValue)
    (`Controller.SetControlRotation` (`self.GetController`) (select `bool` (> ActionValue 0.0) :`false` (`KismetMathLibrary.MakeRotator` 0.0 0.0 -180.0) :`true` (`KismetMathLibrary.MakeRotator` 0.0)))))

(event `self.ReceiveAnyDamage`
  (params (Damage :type "Float (single-precision)") (DamageType :type "DamageType Object Reference") (InstigatedBy :type "Controller Object Reference") (DamageCauser :type "Actor Object Reference"))
  (set `self.Health` (- (`self.Health`) Damage))
  (if (<= (`self.Health`) 0.0)
    (`KismetSystemLibrary.PrintString` "dead")
    (else
      (`KismetSystemLibrary.PrintString` (`KismetStringLibrary.Conv_DoubleToString` (`self.Health`))))))

(event `Key|R`
  (params (Key :type "Key Structure"))
  (:`Pressed`
    (`GameplayStatics.ApplyDamage` self 5.0)))

(event `InputAction|jump`
  (params (Key :type "Key Structure"))
  (:`Pressed`
    (`|PlayMontage` null)))

(event `EnhancedInput|/Game/blueprint/input/Actions/IA_Jump`
  (params (ActionValue :type Boolean) (ElapsedSeconds :type "Float (double-precision)") (TriggeredSeconds :type "Float (double-precision)") (InputAction :type "InputAction Object Reference" :default "/Game/blueprint/input/Actions/IA_Jump.IA_Jump")))

(event `self.OnLanded`
  (params (Hit :type "HitResult Structure (by ref)"))
  (bind _asbp_trex (cast `/Game/blueprint/Trex/BP_Trex` (`.HitActor` (`GameplayStatics.BreakHitResult` Hit))))
  (`self.K2_DestroyActor` _asbp_trex)
  (`self.LaunchCharacter` (* (`KismetMathLibrary.Vector_Up`) (`self.BounceHeight`))))

(fn `Update Animation`
  (bind (_returnvalue_x _returnvalue_y _returnvalue_z) (`KismetMathLibrary.BreakVector` (`self.GetVelocity`)))
  (if (`NavMovementComponent.IsMovingOnGround` (`self.CharacterMovement`))
    (if (> (`KismetMathLibrary.VSize` (`self.GetVelocity`)) 0.0)
      (`PaperFlipbookComponent.SetFlipbook` (`self.Sprite`) "/Game/individual_animations/walk_run/png_sequence/runduck.runduck")
      (else
        (`PaperFlipbookComponent.SetFlipbook` (`self.Sprite`) "/Game/individual_animations/idle/png_sequence/duck.duck")))
    (elif (< _returnvalue_z -80.0)
      (`PaperFlipbookComponent.SetFlipbook` (`self.Sprite`) "/Game/individual_animations/fall/png_sequence/fallduck.fallduck")
      (else
        (`PaperFlipbookComponent.SetFlipbook` (`self.Sprite`) "/Game/individual_animations/jump/png_sequence/jumpduck.jumpduck")))))

(fn `UserConstructionScript`)